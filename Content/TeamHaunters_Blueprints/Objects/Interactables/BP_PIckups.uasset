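; Pickup interactable that shows an interaction prompt while the first-person player character is nearby.
; Overlapping the prompt radius sets the W_PickUpPrompt widget's button icon from the character's UsingGamepad flag (Xbox X or keyboard E) and makes it visible; leaving hides it.
; The input type is checked only when overlap begins, and this graph contains no pickup logic itself.
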(event OnComponentBeginOverlap(Interact_Prompt_Radius)
  (params (OverlappedComponent :type Primitive%20Component%20Object%20Reference) (OtherActor :type Actor%20Object%20Reference) (OtherComp :type Primitive%20Component%20Object%20Reference) (OtherBodyIndex :type Integer) (bFromSweep :type Boolean) (SweepResult :type Hit%20Result%20Structure%20%28by%20ref%29))
  (bind _interaction_prompt (Variables|Default|GetInteraction_Prompt))
  ;[1 1 1] Turns the interact prompt on and off when the player character gets near
  (bind _asbp_gsfpcharacter (Utilities|Casting|CastToBP_GSFPCharacter OtherActor))
  ;;[1 1 1] Checks what kind of controller the player is currently using to output the correct prompt
  (bind _asw_pick_up_prompt (Utilities|Casting|CastToW_PickUpPrompt (UserInterface|GetWidget _interaction_prompt)))
  (if (Variables|/Game/TeamHaunters_Blueprints/Player/BP_GSFPCharacter.BP_GSFPCharacter_C|GetusingGamepad _asbp_gsfpcharacter)
    (Variables|/Game/TeamHaunters_Blueprints/UI/W_PickUpPrompt.W_PickUpPrompt_C|SetButtonPrompt _asw_pick_up_prompt "/Game/TeamHaunters_Assets/Images/Input_Icons/xbox_button_color_x.xbox_button_color_x")
    (else
      (Variables|/Game/TeamHaunters_Blueprints/UI/W_PickUpPrompt.W_PickUpPrompt_C|SetButtonPrompt _asw_pick_up_prompt "/Game/TeamHaunters_Assets/Images/Input_Icons/keyboard_e.keyboard_e")))
  (Rendering|SetVisibility _interaction_prompt true false))

(event OnComponentEndOverlap(Interact_Prompt_Radius)
  (params (OverlappedComponent :type Primitive%20Component%20Object%20Reference) (OtherActor :type Actor%20Object%20Reference) (OtherComp :type Primitive%20Component%20Object%20Reference) (OtherBodyIndex :type Integer))
  ;[1 1 1] Turns the interact prompt on and off when the player character gets near
  (Utilities|Casting|CastToBP_GSFPCharacter OtherActor)
  (Rendering|SetVisibility (Variables|Default|GetInteraction_Prompt) false false))

(fn ConstructionScript)