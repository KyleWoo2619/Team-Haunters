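; BP_Plaque is an interactable plaque that plays narration and serves as one of two triggers for a linked Door event.
; Interact sets the Door's plaque flag, then checks it together with the Door's casket flag.
; When both are set, a long delay precedes a door-closing sound and the Door's SetPhysics call.
; A short delay later, zombie-area ambience and a noise-heard narration line play.
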(event EventInteract
  (params (Player :type Object%20Object%20Reference))
  (bind _door (Variables|Default|GetDoor))
  (Audio|PlaySound2D "/Game/TeamHaunters_Assets/Sound/Haunters_Brandon/Narration/NAR_interact_with_plaque.NAR_interact_with_plaque" 1.0 1.0 0.0 0 0)
  (Variables|/Game/TeamHaunters_Blueprints/Objects/Extra/BP_MausoleumDoor.BP_MausoleumDoor_C|SetPlaqueInteracted _door true)
  (if (and (Variables|/Game/TeamHaunters_Blueprints/Objects/Extra/BP_MausoleumDoor.BP_MausoleumDoor_C|GetPlaqueInteracted _door) (Variables|/Game/TeamHaunters_Blueprints/Objects/Extra/BP_MausoleumDoor.BP_MausoleumDoor_C|GetCasketInteracted _door))
    (Utilities|FlowControl|Delay 13.31)
    (Audio|PlaySound2D "/Game/TeamHaunters_Assets/Sound/Extra/close-door-sound-247450.close-door-sound-247450" 1.0 1.0 0.0 0 0)
    (Default|SetPhysics _door)
    (Utilities|FlowControl|Delay 1.0)
    (Audio|PlaySound2D "/Game/TeamHaunters_Assets/Sound/Haunters_Brandon/NotUsed/NU_zombie_area_sfx.NU_zombie_area_sfx" 1.0 1.0 0.0 0 0)
    (Audio|PlaySound2D "/Game/TeamHaunters_Assets/Sound/Haunters_Brandon/Narration/NAR_noise-is-heard.NAR_noise-is-heard" 1.0 1.0 0.0 0 0)))

(fn ConstructionScript)