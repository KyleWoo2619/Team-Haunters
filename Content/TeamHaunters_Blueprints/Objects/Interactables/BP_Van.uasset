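; BP_Van is the interactable van that ends the level once the player has both the key and the gas jug.
; With both items, it disables input once, teleports the player, shows two Niagara effects and calls the end-level event.
; Otherwise it plays a failed-start or locked-door sound, plus narration the first time each missing-item case occurs.
; Every failed attempt also makes noise at the player's location.
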(event EventInteract
  (params (Player :type Object%20Object%20Reference))
  (bind _asbp_gsfpcharacter (Utilities|Casting|CastToBP_GSFPCharacter (Game|GetPlayerCharacter 0)))
  (if (and (Variables|/Game/TeamHaunters_Blueprints/Player/BP_GSFPCharacter.BP_GSFPCharacter_C|GetHasKey _asbp_gsfpcharacter) (Variables|/Game/TeamHaunters_Blueprints/Player/BP_GSFPCharacter.BP_GSFPCharacter_C|GetHasJug _asbp_gsfpcharacter))
    (Utilities|FlowControl|DoOnce false
      (:Completed
        (Input|DisableInput _asbp_gsfpcharacter 0)
        (Transformation|SetActorTransform _asbp_gsfpcharacter (Math|Transform|MakeTransform "0, 0, 0" "0, 0, 0" "1.000000,1.000000,1.000000") false true)
        (Rendering|SetVisibility (Variables|Default|GetNiagara1) true false)
        (Default|CallEndLevel)))
    (elif (Variables|/Game/TeamHaunters_Blueprints/Player/BP_GSFPCharacter.BP_GSFPCharacter_C|GetHasKey _asbp_gsfpcharacter)
      (if (not (Variables|/Game/TeamHaunters_Blueprints/Player/BP_GSFPCharacter.BP_GSFPCharacter_C|GetHasJug _asbp_gsfpcharacter))
        (Audio|PlaySound2D "/Game/TeamHaunters_Assets/Sound/Extra/failed-car-start.failed-car-start" 1.0 1.0 0.0 0 0)
        (if (Variables|Default|GetKeyNoGas)
          _
          (else
            (Variables|Default|SetKeyNoGas true)
            (Audio|PlaySound2D "/Game/TeamHaunters_Assets/Sound/Haunters_Brandon/Narration/NAR_key__no_gas.NAR_key__no_gas" 1.0 1.0 0.0 0 0)))
        (Class|Actor|MakeNoise 1.0 0 (Transformation|GetActorLocation _asbp_gsfpcharacter) 0.0 "None" :!label _label))
      (elif (Variables|/Game/TeamHaunters_Blueprints/Player/BP_GSFPCharacter.BP_GSFPCharacter_C|GetHasJug _asbp_gsfpcharacter)
        (Audio|PlaySound2D "/Game/TeamHaunters_Assets/Sound/Haunters_Brandon/try_to_open_door.try_to_open_door" 1.0 1.0 0.0 0 0)
        (if (Variables|Default|GetNoKeyGas)
          (goto _label)
          (else
            (Variables|Default|SetNoKeyGas true)
            (Audio|PlaySound2D "/Game/TeamHaunters_Assets/Sound/Haunters_Brandon/Narration/NAR_gas__no_key.NAR_gas__no_key" 1.0 1.0 0.0 0 0)
            (goto _label)))
        (else
          (Audio|PlaySound2D "/Game/TeamHaunters_Assets/Sound/Haunters_Brandon/try_to_open_door.try_to_open_door" 1.0 1.0 0.0 0 0)
          (if (Variables|Default|GetNoKeyNoGas)
            (goto _label)
            (else
              (Variables|Default|SetNoKeyNoGas true)
              (Audio|PlaySound2D "/Game/TeamHaunters_Assets/Sound/Haunters_Brandon/Narration/NAR_no_key_no_gas.NAR_no_key_no_gas" 1.0 1.0 0.0 0 0)
              (goto _label))))))))

(fn ConstructionScript)