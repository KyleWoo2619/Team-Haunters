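; BP_Hide is an interactable hiding spot that moves the first-person player in and out of cover.
; Interacting to hide disables player collision and movement, and a looping timer at frame delta slides the player at constant speed to PlayerPosition, or to ExitPosition when leaving.
; On arrival, the timers clear and the player's hiding and crouching flags flip, with collision and walking restored on exit.
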(event Custom|MoveCharacter
  (bind _playerref (Variables|Default|GetPlayerRef))
  (bind _playerref_2 (Variables|Default|GetPlayerRef))
  (bind _is_hiding (Variables|/Game/FirstPerson/Blueprints/BP_FirstPersonCharacter.BP_FirstPersonCharacter_C|GetIs%20Hiding _playerref_2))
  ;[1 1 1] Disabling movement
  ;[1 1 1] Placing player in the hide
  (Transformation|SetActorTransform _playerref (Math|Transform|MakeTransform (Math|Interpolation|VInterptoConstant (Transformation|GetActorLocation _playerref) (Transformation|GetWorldLocation (select _is_hiding (Variables|Default|GetExitPosition) (Variables|Default|GetPlayerPosition))) (Utilities|Time|GetWorldDeltaSeconds) 1e+03) "0, 0, 0" "1.000000,1.000000,1.000000"))
  (if (Utilities|Operators|EqualEqual (Transformation|GetActorLocation (Variables|Default|GetPlayerRef)) (Transformation|GetWorldLocation (select _is_hiding (Variables|Default|GetExitPosition) (Variables|Default|GetPlayerPosition))) 0.01)
    (Utilities|Time|ClearandInvalidateTimerbyHandle (stale EventInteract _returnvalue_2))
    (Utilities|Time|ClearandInvalidateTimerbyHandle (stale EventInteract _returnvalue))
    (CallFunction|FinishedHiding)))

(event Custom|Finished%20Hiding
  (bind _playerref (Variables|Default|GetPlayerRef))
  ;[1 1 1] Hiding check
  (if (Variables|/Game/FirstPerson/Blueprints/BP_FirstPersonCharacter.BP_FirstPersonCharacter_C|GetIs%20Hiding _playerref)
    (Variables|/Game/FirstPerson/Blueprints/BP_FirstPersonCharacter.BP_FirstPersonCharacter_C|SetIs%20Hiding _playerref false)
    (Variables|/Game/FirstPerson/Blueprints/BP_FirstPersonCharacter.BP_FirstPersonCharacter_C|SetIsCrouching _playerref false)
    (Collision|SetActorEnableCollision _playerref true)
    (Pawn|Components|CharacterMovement|SetMovementMode (Variables|/Script/Engine.Character|GetCharacterMovement _playerref) "MOVE_Walking" 0)
    (else
      (Variables|/Game/FirstPerson/Blueprints/BP_FirstPersonCharacter.BP_FirstPersonCharacter_C|SetIs%20Hiding _playerref true)
      (Variables|/Game/FirstPerson/Blueprints/BP_FirstPersonCharacter.BP_FirstPersonCharacter_C|SetIsCrouching _playerref true))))

(event EventBeginPlay
  ;[1 1 1] Getting Player
  (bind _asbp_first_person_character (Utilities|Casting|CastToBP_FirstPersonCharacter (Game|GetPlayerCharacter 0)))
  (Variables|Default|SetPlayerRef _asbp_first_person_character))

(event EventInteract
  (bind _playerref (Variables|Default|GetPlayerRef))
  ;[1 1 1] Interacted
  (if (Variables|/Game/FirstPerson/Blueprints/BP_FirstPersonCharacter.BP_FirstPersonCharacter_C|GetIs%20Hiding (Variables|Default|GetPlayerRef))
    (bind _returnvalue (Utilities|Time|SetTimerbyEvent (delegate Custom|MoveCharacter) (Utilities|Time|GetWorldDeltaSeconds) true))
    (else
      ;[1 1 1] Disabling movement
      (Collision|SetActorEnableCollision _playerref false)
      (Pawn|Components|CharacterMovement|DisableMovement (Variables|/Script/Engine.Character|GetCharacterMovement _playerref))
      (bind _returnvalue_2 (Utilities|Time|SetTimerbyEvent (delegate Custom|MoveCharacter) (Utilities|Time|GetWorldDeltaSeconds) true)))))

(fn ConstructionScript)