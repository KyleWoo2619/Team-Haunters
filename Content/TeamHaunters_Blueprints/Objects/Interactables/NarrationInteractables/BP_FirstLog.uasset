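; BP_FirstLog is an interactable log hiding spot that plays a one-time narration the first time the player hides in it.
; Interact toggles between entering and exiting, disabling collision and movement on entry and switching HideMesh lighting channels off while hidden.
; A per-frame looping timer glides the player to the hide or exit point with VInterpToConstant.
; On arrival it flips the player's hiding and crouching flags, restoring collision and walking on exit.
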(event Custom|MoveCharacter
  (bind _playerref (Variables|Default|GetPlayerRef))
  (bind _playerref_2 (Variables|Default|GetPlayerRef))
  (bind _ishiding (Variables|/Game/TeamHaunters_Blueprints/Player/BP_GSFPCharacter.BP_GSFPCharacter_C|GetIsHiding _playerref_2))
  ;[1 1 1] Disabling movement
  ;[1 1 1] Placing player in the hide
  (Transformation|SetActorTransform _playerref (Math|Transform|MakeTransform (Math|Interpolation|VInterptoConstant (Transformation|GetActorLocation _playerref) (Transformation|GetWorldLocation (select _ishiding (Variables|Default|GetExitPosition) (Variables|Default|GetPlayerPosition))) (Utilities|Time|GetWorldDeltaSeconds) 1e+03) "0, 0, 0" "1.000000,1.000000,1.000000"))
  (if (Utilities|Operators|EqualEqual (Transformation|GetActorLocation (Variables|Default|GetPlayerRef)) (Transformation|GetWorldLocation (select _ishiding (Variables|Default|GetExitPosition) (Variables|Default|GetPlayerPosition))) 0.01)
    (Utilities|Time|ClearandInvalidateTimerbyHandle (stale EventInteract _returnvalue_2))
    (Utilities|Time|ClearandInvalidateTimerbyHandle (stale EventInteract _returnvalue))
    (CallFunction|FinishedHiding)))

(event Custom|Finished%20Hiding
  (bind _playerref (Variables|Default|GetPlayerRef))
  ;[1 1 1] Hiding check
  (if (Variables|/Game/TeamHaunters_Blueprints/Player/BP_GSFPCharacter.BP_GSFPCharacter_C|GetIsHiding _playerref)
    (Variables|/Game/TeamHaunters_Blueprints/Player/BP_GSFPCharacter.BP_GSFPCharacter_C|SetIsHiding _playerref false)
    (Variables|/Game/TeamHaunters_Blueprints/Player/BP_GSFPCharacter.BP_GSFPCharacter_C|SetIsCrouching _playerref false)
    (Collision|SetActorEnableCollision _playerref true)
    (Pawn|Components|CharacterMovement|SetMovementMode (Variables|/Script/Engine.Character|GetCharacterMovement _playerref) "MOVE_Walking" 0)
    (else
      (Variables|/Game/TeamHaunters_Blueprints/Player/BP_GSFPCharacter.BP_GSFPCharacter_C|SetIsHiding _playerref true)
      (Variables|/Game/TeamHaunters_Blueprints/Player/BP_GSFPCharacter.BP_GSFPCharacter_C|SetIsCrouching _playerref true))))

(event EventBeginPlay
  ;[1 1 1] Getting Player
  (bind _asbp_gsfpcharacter (Utilities|Casting|CastToBP_GSFPCharacter (Game|GetPlayerCharacter 0)))
  (Variables|Default|SetPlayerRef _asbp_gsfpcharacter))

(event EventInteract
  (params (Player :type Object%20Object%20Reference))
  (bind _playerref (Variables|Default|GetPlayerRef))
  ;[1 1 1] Interacted
  (Rendering|Components|SetLightingChannels (Variables|Default|GetHideMesh) false false false)
  (if (Variables|/Game/TeamHaunters_Blueprints/Player/BP_GSFPCharacter.BP_GSFPCharacter_C|GetIsHiding (Variables|Default|GetPlayerRef))
    (bind _returnvalue (Utilities|Time|SetTimerbyEvent (delegate Custom|MoveCharacter) (Utilities|Time|GetWorldDeltaSeconds) true))
    (Rendering|Components|SetLightingChannels (Variables|Default|GetHideMesh) true true true)
    (else
      ;[1 1 1] Disabling movement
      (if (Variables|Default|GetHasTriggered)
        _
        (else
          (Variables|Default|SetHasTriggered true)
          (Audio|SpawnSound2D "/Game/TeamHaunters_Assets/Sound/Haunters_Brandon/Narration/NAR_hiding_in_log.NAR_hiding_in_log" 1.0 1.0 0.0 0)))
      (Collision|SetActorEnableCollision _playerref false)
      (Pawn|Components|CharacterMovement|DisableMovement (Variables|/Script/Engine.Character|GetCharacterMovement _playerref))
      (bind _returnvalue_2 (Utilities|Time|SetTimerbyEvent (delegate Custom|MoveCharacter) (Utilities|Time|GetWorldDeltaSeconds) true)))))

(fn ConstructionScript)