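; BP_Key is a blue or red key pickup that unlocks a linked door when its static mesh is overlapped.
; On BeginPlay each key creates both key HUD widgets and adds them to the viewport hidden.
; Any overlap plays a coin sound at the world origin.
; If the Blue or Red flag is set, it shows the matching widget, calls SetPhysics on DoorToOpen and destroys itself.
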(event OnComponentBeginOverlap(StaticMesh)
  (params (OverlappedComponent :type Primitive%20Component%20Object%20Reference) (OtherActor :type Actor%20Object%20Reference) (OtherComp :type Primitive%20Component%20Object%20Reference) (OtherBodyIndex :type Integer) (bFromSweep :type Boolean) (SweepResult :type Hit%20Result%20Structure%20%28by%20ref%29))
  (Audio|PlaySoundatLocation "/Game/TeamHaunters_Import/Sound/Extra/CoinSound.CoinSound" "0, 0, 0" "0, 0, 0" 1.0 1.0 0.0 0 0 0 0)
  (if (Variables|Default|GetBlue)
    (Variables|Default|SetBlueKey (Variables|Default|GetBlueKey))
    (Widget|SetVisibility (Variables|Default|GetBlueKey) "Visible")
    (Default|SetPhysics (Variables|Default|GetDoorToOpen))
    (Actor|DestroyActor)
    (elif (Variables|Default|GetRed)
      (Variables|Default|SetRedKey (Variables|Default|GetRedKey))
      (Widget|SetVisibility (Variables|Default|GetRedKey) "Visible")
      (Default|SetPhysics (Variables|Default|GetDoorToOpen))
      (Actor|DestroyActor))))

(event EventBeginPlay
  (Utilities|FlowControl|Sequence
    (:then_0
      (bind _returnvalue (UserInterface|CreateWidget "/Game/TeamHaunters_Blueprints/UI/WG_BlueKey.WG_BlueKey_C" (Game|GetPlayerController 0)))
      (bind _output_get (Variables|Default|SetBlueKey _returnvalue))
      (UserInterface|Viewport|AddtoViewport _output_get 0)
      (Widget|SetVisibility _output_get "Hidden"))
    (:then_1
      (bind _returnvalue_2 (UserInterface|CreateWidget "/Game/TeamHaunters_Blueprints/UI/WG_RedKey.WG_RedKey_C" (Game|GetPlayerController 0)))
      (bind _output_get_2 (Variables|Default|SetRedKey _returnvalue_2))
      (UserInterface|Viewport|AddtoViewport _output_get_2 0)
      (Widget|SetVisibility _output_get_2 "Hidden"))))

(fn ConstructionScript)