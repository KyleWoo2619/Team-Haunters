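; BP_EnemyBase is an enemy character Blueprint that provides patrol route access, movement speed control and a level restart event.
; GetPatrolRoute returns the stored route, while SetMovementSpeed maps a patrol, jogging or chase state to the CharacterMovement max walk speed and returns it.
; RestartGame prints the current level name and reopens that level by name.
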(event Custom|RestartGame
  (bind _returnvalue (Game|GetCurrentLevelName true))
  (Development|PrintString _returnvalue)
  (Game|OpenLevel(byName) (Utilities|String|StringToName _returnvalue)))

(fn ConstructionScript)

(fn GetPatrolRoute
  (return (Variables|AI|GetPatrolRoute)))

(fn SetMovementSpeed
  (params (Speed :type E_MovementSpeed%20Enum :default "NewEnumerator0"))
  (bind _output_get (Variables|/Script/Engine.CharacterMovementComponent|SetMaxWalkSpeed (Variables|Character|GetCharacterMovement) (Utilities|Select :Index Speed :NewEnumerator0 1e+02 :NewEnumerator1 3e+02 :NewEnumerator2 2e+02)))
  (return _output_get))